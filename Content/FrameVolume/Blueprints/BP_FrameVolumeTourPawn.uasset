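; BP_FrameVolumeTourPawn is a pawn that automatically tours back and forth along the X axis, apparently for showcasing frame volumes.
; Each tick it moves at Speed on a fixed Y and height, flipping Dir when the next step would pass MinX or MaxX.
; Its yaw snaps to face the travel direction, without sweep or interpolation.
; PauseTour and ResumeTour events toggle the movement.
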(event Custom|PauseTour
  (Variables|FrameVolumeDemoTour|SetbTourPaused true))

(event Custom|ResumeTour
  (Variables|FrameVolumeDemoTour|SetbTourPaused false))

(event EventTick
  (params (DeltaSeconds :type Float%20%28single-precision%29))
  (if (not (Variables|FrameVolumeDemoTour|GetbTourPaused))
    (if (> (+ (.X (Math|Vector|BreakVector (Transformation|GetActorLocation))) (* (* (Variables|FrameVolumeDemoTour|GetDir) (Variables|FrameVolumeDemoTour|GetSpeed)) DeltaSeconds)) (Variables|FrameVolumeDemoTour|GetMaxX))
      (Variables|FrameVolumeDemoTour|SetDir -1.0)
      (elif (< (+ (.X (Math|Vector|BreakVector (Transformation|GetActorLocation))) (* (* (Variables|FrameVolumeDemoTour|GetDir) (Variables|FrameVolumeDemoTour|GetSpeed)) DeltaSeconds)) (Variables|FrameVolumeDemoTour|GetMinX))
        (Variables|FrameVolumeDemoTour|SetDir 1.0)))
    (Transformation|SetActorLocation (Math|Vector|MakeVector (+ (.X (Math|Vector|BreakVector (Transformation|GetActorLocation))) (* (* (Variables|FrameVolumeDemoTour|GetDir) (Variables|FrameVolumeDemoTour|GetSpeed)) DeltaSeconds)) 0.0 1.1e+02) false false)
    (if (> (Variables|FrameVolumeDemoTour|GetDir) (Math|Float|MakeLiteralFloat 0.0))
      (Transformation|SetActorRotation (Math|Rotator|MakeRotator 0.0 0.0 0.0))
      (else
        (Transformation|SetActorRotation (Math|Rotator|MakeRotator 0.0 0.0 1.8e+02))))))

(fn ConstructionScript)